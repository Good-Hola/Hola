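; AI controller for the Fat Monster that runs BT_Monster and feeds its blackboard.
; BeginPlay caches the pawn, seeds patrol looping, direction and wait time from its PatrolPath, stores the player as target and writes the initial ChaseStatus.
; AI perception sets CanSeePlayer on sensing updates for the player, while PawnAttack forwards to the pawn's Attack.
; A one-shot timer runs a Test event that overrides ChaseStatus shortly after start.
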(event OnTargetPerceptionUpdated(AIPerception)
  (params (Actor :type Actor%20Object%20Reference) (Stimulus :type AI%20Stimulus%20Structure))
  (Utilities|Casting|CastToPlayerCharacter Actor)
  (AI|Components|Blackboard|SetValueasBool (AI|GetBlackboard 0) (Utilities|Name|MakeLiteralName "CanSeePlayer") (.bSuccessfullySensed (Utilities|Struct|BreakAIStimulus Stimulus))))

(event Custom|PawnAttack
  (Default|Attack (Variables|Default|GetMyPawn)))

(event Custom|Test
  (bind _output_get (Variables|Default|SetCurrentState "NewEnumerator3"))
  (AI|Components|Blackboard|SetValueasEnum (AI|GetBlackboard 0) (Utilities|Name|MakeLiteralName "ChaseStatus") _output_get))

(event EventBeginPlay
  (bind _returnvalue (AI|GetBlackboard 0))
  (AI|RunBehaviorTree "/Game/AI/AI/BT_Monster.BT_Monster")
  (bind _asbp_fat_monster (Utilities|Casting|CastToBP_Fat_Monster (Pawn|GetControlledPawn)))
  (bind _output_get (Variables|Default|SetMyPawn _asbp_fat_monster))
  (AI|Components|Blackboard|SetValueasBool (AI|GetBlackboard 0) (Utilities|Name|MakeLiteralName "PathLooping") (Variables|/Game/AI/AI/PatrolPath.PatrolPath_C|GetisLooping (Variables|/Game/AI/AI/BP_Fat_Monster.BP_Fat_Monster_C|GetPatrolPath _output_get)))
  (Class|BlackboardComponent|SetValueasInt _returnvalue (Utilities|Name|MakeLiteralName "Direction") 1)
  (AI|Components|Blackboard|SetValueasFloat _returnvalue (Utilities|Name|MakeLiteralName "WaitTime") (Variables|/Game/AI/AI/PatrolPath.PatrolPath_C|GetWaitTime (Variables|/Game/AI/AI/BP_Fat_Monster.BP_Fat_Monster_C|GetPatrolPath (Variables|Default|GetMyPawn))))
  (Variables|Default|SetCurrentTarget (Game|GetPlayerCharacter 0))
  (AI|Components|Blackboard|SetValueasEnum _returnvalue (Utilities|Name|MakeLiteralName "ChaseStatus") (Variables|Default|GetCurrentState))
  (Utilities|Time|SetTimerbyEvent (delegate Custom|Test) 4.0))

(fn ConstructionScript)