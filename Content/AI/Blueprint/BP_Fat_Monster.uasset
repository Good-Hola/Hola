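; BP_Fat_Monster is an enemy monster with a melee attack that damages the player.
; MeleeAttack plays a right-hand attack montage and waits for its notify to time the hit.
; On the notify, a short sphere trace runs forward from the right hand socket on the Visibility channel.
; The hit actor, cast to PlayerCharacter, receives the Damage value, followed by a debug "Hit" print.
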(event OnComponentHit(CapsuleComponent)
  (params (HitComponent :type Primitive%20Component%20Object%20Reference) (OtherActor :type Actor%20Object%20Reference) (OtherComp :type Primitive%20Component%20Object%20Reference) (NormalImpulse :type Vector :default "0, 0, 0") (Hit :type Hit%20Result%20Structure%20%28by%20ref%29)))

(event EventMeleeAttack
  (bind _mesh (Variables|Character|GetMesh))
  (bind _returnvalue (Transformation|GetSocketLocation _mesh "hand_r_socket"))
  (Animation|Montage|PlayMontage (Variables|Character|GetMesh) "/Game/AI/Animations/Anim_attack_1_r_Montage.Anim_attack_1_r_Montage"
    (:OnNotifyBegin
      (bind _outhit (Collision|SphereTraceByChannel _returnvalue (+ _returnvalue (* (Math|Vector|GetForwardVector (Transformation|GetActorRotation)) 5e+01)) 4e+01 "TraceTypeQuery1" false 0 "None"))
      (Game|Damage|ApplyDamage (.AsPlayer%20Character (Utilities|Casting|CastToPlayerCharacter (.hitactor _outhit))) (Variables|AI|GetDamage) 0 0)
      (Development|PrintString "Hit"))))

(fn ConstructionScript)