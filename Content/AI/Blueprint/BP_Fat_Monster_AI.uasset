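; AI controller for the fat monster that runs its behavior tree and feeds perception results into the blackboard.
; On BeginPlay it seeds patrol settings from the pawn's PatrolPath, stores the player as target and writes the initial chase state.
; Perception updates go to Sensing, which treats stimuli by array index: the first sets CanSeePlayer, while a successful second or third flags investigation at the stimulus location.
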(event OnPerceptionUpdated(AIPerception)
  (params (UpdatedActors :type Array%20of%20Actor%20Object%20References))
  (for _array_element UpdatedActors
    (bind _info (Class|AIPerceptionComponent|GetActorsPerception (Variables|Default|GetAIPerception) _array_element))
    (CallFunction|Sensing (.lastsensedstimuli _info))))

(event EventBeginPlay
  (bind _returnvalue (AI|GetBlackboard 0))
  (AI|RunBehaviorTree "/Game/AI/AI/BT_Monster.BT_Monster")
  (bind _asbp_fat_monster (Utilities|Casting|CastToBP_Fat_Monster (Pawn|GetControlledPawn)))
  (bind _output_get (Variables|Default|SetMyPawn _asbp_fat_monster))
  (AI|Components|Blackboard|SetValueasBool (AI|GetBlackboard 0) (Utilities|Name|MakeLiteralName "PathLooping") (Variables|/Game/AI/Blueprint/PatrolPath.PatrolPath_C|GetisLooping (Variables|/Game/AI/Blueprint/BP_Fat_Monster.BP_Fat_Monster_C|GetPatrolPath _output_get)))
  (Class|BlackboardComponent|SetValueasInt _returnvalue (Utilities|Name|MakeLiteralName "Direction") 1)
  (AI|Components|Blackboard|SetValueasFloat _returnvalue (Utilities|Name|MakeLiteralName "WaitTime") (Variables|/Game/AI/Blueprint/PatrolPath.PatrolPath_C|GetWaitTime (Variables|/Game/AI/Blueprint/BP_Fat_Monster.BP_Fat_Monster_C|GetPatrolPath (Variables|Default|GetMyPawn))))
  (Variables|Default|SetCurrentTarget (Game|GetPlayerCharacter 0))
  (AI|Components|Blackboard|SetValueasEnum _returnvalue (Utilities|Name|MakeLiteralName "ChaseStatus") (Variables|Default|GetCurrentState)))

(fn ConstructionScript)

(fn Sensing
  (params (Array :type Array%20of%20AI%20Stimulus%20Structures))
  (bind _returnvalue (AI|GetBlackboard 0))
  (for (_array_element _array_index) Array
    (LocalVariables|SetlocalSensing _array_element)
    (switch int _array_index
      (:0
        (AI|Components|Blackboard|SetValueasBool (AI|GetBlackboard 0) (Utilities|Name|MakeLiteralName "CanSeePlayer") (.bsuccessfullysensed (LocalVariables|GetlocalSensing))))
      (:1
        (if (.bsuccessfullysensed (LocalVariables|GetlocalSensing)) :!label _label
          (AI|Components|Blackboard|SetValueasBool _returnvalue (Utilities|Name|MakeLiteralName "IsInvestigating") (.bsuccessfullysensed (LocalVariables|GetlocalSensing)))
          (AI|Components|Blackboard|SetValueasVector _returnvalue (Utilities|Name|MakeLiteralName "Location") (.stimuluslocation (LocalVariables|GetlocalSensing)))))
      (:2
        (goto _label)))))