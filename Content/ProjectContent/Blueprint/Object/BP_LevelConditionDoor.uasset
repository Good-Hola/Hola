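; BP_LevelConditionDoor is a sci-fi door that opens only when the player character's CurrentStage is at least its Level value.
; Trigger overlaps filter for the player's trigger capsule by comparing a hard-coded display name.
; Entry plays a sound, activates two steam components and runs a timeline that lerps DoorSmallA open.
; Exit replays the sound and reverses the timeline, but checks a fixed stage 3 instead of Level.
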(event OnComponentBeginOverlap(Trigger)
  (params (OverlappedComponent :type Primitive%20Component%20Object%20Reference) (OtherActor :type Actor%20Object%20Reference) (OtherComp :type Primitive%20Component%20Object%20Reference) (OtherBodyIndex :type Integer) (bFromSweep :type Boolean) (SweepResult :type Hit%20Result%20Structure%20%28by%20ref%29))
  (bind _asplayer_character (Utilities|Casting|CastToPlayerCharacter OtherActor))
  (if (and (>= (Variables|/Script/Hola.PlayerCharacter|GetcurrentStage _asplayer_character) (Variables|Default|Getlevel)) (Utilities|Enum|Equal(Enum) (Utilities|GetDisplayName OtherComp) "BP_PlayerCharacter_C_0.Trigger Capsule"))
    (Audio|PlaySoundatLocation "/Game/ProjectContent/Sounds/SoundCue/Cue_SciFiDoor.Cue_SciFiDoor" (Variables|/Script/Engine.SceneComponent|GetRelativeLocation (Variables|Default|GetDefaultSceneRoot)) "0, 0, 0" 1.0 1.0 0.0 0 0 0)
    (Components|Activation|Activate (Variables|Default|GetSteamDoor) false)
    (bind _doorposition (Timeline|Timeline_0 Play)
      (:Update
        (Transformation|SetRelativeLocation (Variables|Default|GetDoor_Small_A) (Math|Vector|Lerp(Vector) (Variables|Door|GetDoorClosed) (Variables|Door|GetDoorOpen) _doorposition) false false)))))

(event OnComponentEndOverlap(Trigger)
  (params (OverlappedComponent :type Primitive%20Component%20Object%20Reference) (OtherActor :type Actor%20Object%20Reference) (OtherComp :type Primitive%20Component%20Object%20Reference) (OtherBodyIndex :type Integer))
  (bind _asplayer_character (Utilities|Casting|CastToPlayerCharacter OtherActor))
  (if (and (>= (Variables|/Script/Hola.PlayerCharacter|GetcurrentStage _asplayer_character) 3) (Utilities|Enum|Equal(Enum) (Utilities|GetDisplayName OtherComp) "BP_PlayerCharacter_C_0.Trigger Capsule"))
    (Audio|PlaySoundatLocation "/Game/ProjectContent/Sounds/SoundCue/Cue_SciFiDoor.Cue_SciFiDoor" (Variables|/Script/Engine.SceneComponent|GetRelativeLocation (Variables|Default|GetDefaultSceneRoot)) "0, 0, 0" 1.0 1.0 0.0 0 0 0)
    (bind _doorposition (Timeline|Timeline_0 Reverse)
      (:Update
        (Transformation|SetRelativeLocation (Variables|Default|GetDoor_Small_A) (Math|Vector|Lerp(Vector) (Variables|Door|GetDoorClosed) (Variables|Door|GetDoorOpen) _doorposition) false false)))))

(fn ConstructionScript)