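; Password puzzle manager that collects entered digits and moves the character to stage 4 when the code is correct.
; AddPassword appends each digit and runs CheckPassword, which at six entries combines them by place value and compares against CorrectPassword; the sixth is multiplied by zero, so it never counts.
; A wrong code clears the entry and resets every linked button's light and active flag.
; ChangeStatus sets stage 4 without any check.
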(event Custom|커스텀이벤트_0)

(fn ConstructionScript)

(fn AddPassword
  (params (NewPass :type Integer) (character :type Player%20Character%20Object%20Reference))
  (Utilities|Array|Add (Variables|Default|GetPassword) NewPass)
  (CallFunction|CheckPassword character))

(fn CheckPassword
  (params (character :type Player%20Character%20Object%20Reference))
  (if (== (Utilities|Array|Length (Variables|Default|GetPassword)) 6)
    (if (== (+ (* (Utilities|Array|Get(acopy) (Variables|Default|GetPassword)) 100000) (* (Utilities|Array|Get(acopy) (Variables|Default|GetPassword) 1) 10000) (* (Utilities|Array|Get(acopy) (Variables|Default|GetPassword) 2) 1000) (* (Utilities|Array|Get(acopy) (Variables|Default|GetPassword) 3) 100) (* (Utilities|Array|Get(acopy) (Variables|Default|GetPassword) 4) 10) (* (Utilities|Array|Get(acopy) (Variables|Default|GetPassword) 5) 0)) (Variables|Default|GetCorrectPassword))
      (Variables|/Script/Hola.PlayerCharacter|SetcurrentStage character 4)
      (Development|PrintString "Complete")
      (else
        (Utilities|Array|Clear (Variables|Default|GetPassword))
        (for _array_element (Variables|Default|GetButtons)
          (Default|ChangeLight _array_element)
          (Variables|/Script/Hola.InteractObject|SetisAct _array_element false)
          (Development|PrintString "Failed"))))))

(fn ChangeStatus
  (params (character :type Player%20Character%20Object%20Reference))
  (if true
    (Variables|/Script/Hola.PlayerCharacter|SetcurrentStage character 4)))