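; BP_SaveAndLoadGameMode is a game mode Blueprint that saves and restores the player pawn's transform.
; Saving writes the pawn's transform into a new BP_SaveData object stored in the "PlayerTransform" slot.
; Loading reads that slot, casts it to BP_SaveData and applies the transform to the pawn without sweep or teleport.
; SaveAll and LoadAll wrap these functions as general entry points, currently covering only the transform.
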(fn ConstructionScript)

(fn PlayerTransformSave
  (bind _returnvalue (SaveGame|CreateSaveGameObject "/Game/ProjectContent/Blueprint/SaveGame/BP_SaveData.BP_SaveData_C"))
  (Default|SetPlayerTransform _returnvalue (Transformation|GetActorTransform (Game|Player|GetPlayerPawn 0)))
  (SaveGame|SaveGametoSlot _returnvalue "PlayerTransform"))

(fn PlayerTransformLoad
  (bind _returnvalue (SaveGame|LoadGamefromSlot "PlayerTransform"))
  (bind _asbp_save_data (Utilities|Casting|CastToBP_SaveData _returnvalue))
  (Transformation|SetActorTransform (Game|Player|GetPlayerPawn 0) (Variables|/Game/ProjectContent/Blueprint/SaveGame/BP_SaveData.BP_SaveData_C|GetPlayerTransform _asbp_save_data)))

(fn SaveAll
  (CallFunction|PlayerTransformSave))

(fn LoadAll
  (CallFunction|PlayerTransformLoad))