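; BP_TestPlayer is a test player character Blueprint that handles jump and crouch input.
; Jump sets IsInAir while held, and crouching requires both that flag to be clear and the movement component not to be falling.
; Releasing crouch runs a capsule trace built from scaled capsule world location, re-crouching on initial overlap and otherwise standing up.
; BeginPlay, overlap, Tick and the construction script are empty.
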(event EventBeginPlay)

(event Collision|EventActorBeginOverlap
  (params (OtherActor :type Actor%20Object%20Reference)))

(event EventTick
  (params (DeltaSeconds :type Float%20%28single-precision%29)))

(event Input|ActionEvents|InputActionCrouch
  (params (Key :type Key%20Structure :default "None"))
  (bind _capsulecomponent (Variables|Default|GetCapsuleComponent))
  (bind _returnvalue (Transformation|GetWorldLocation _capsulecomponent))
  (bind _returnvalue_2 (* _returnvalue 200))
  (:Pressed
    (if (and (not (Variables|Default|GetIsInAir?)) (not (AI|Components|NavMovement|IsFalling (Variables|Character|GetCharacterMovement))))
      (Character|Crouch :!label _label)
      (Variables|Default|SetisCrouching true)))
  (:Released
    (bind _outhit (Collision|CapsuleTraceByChannel (+ (Transformation|GetWorldLocation _capsulecomponent) _returnvalue_2) _returnvalue_2 0.0 0.0 "TraceTypeQuery1" false 0 "None"))
    (if (.bInitialOverlap (Collision|BreakHitResult _outhit))
      (goto _label)
      (else
        (Character|UnCrouch)
        (Variables|Default|SetisCrouching false)))))

(event Input|ActionEvents|InputActionJump
  (params (Key :type Key%20Structure :default "None"))
  (:Pressed
    (Variables|Default|SetIsInAir? true)
    (Character|Jump))
  (:Released
    (Variables|Default|SetIsInAir? false)
    (Character|StopJumping)))

(fn ConstructionScript)