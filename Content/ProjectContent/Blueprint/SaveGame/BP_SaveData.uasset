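; BP_SaveData is a save game Blueprint meant to store player stats, weapons, and interact object and enemy states in the "GameData" slot.
; Update events fill per-index arrays, but only interact object transforms receive real values, and the player and weapon assignments are unwired.
; Save writes a newly created instance instead of the updated one.
; Load reads and casts the slot's data without applying it.
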(event Custom|Load
  (bind _returnvalue (SaveGame|LoadGamefromSlot "GameData"))
  (bind _asbp_save_data (Utilities|Casting|CastToBP_SaveData _returnvalue)))

(event Custom|ChangeWeapon
  (params (HandWeapon :type Integer) (BackWeapon :type Integer)))

(event Custom|UpdatePlayerInfo
  (params (PlayerHp :type Float%20%28single-precision%29) (PlayerTransform :type Transform) (PlayerEnergy :type Float%20%28single-precision%29)))

(event Custom|UpdateInteractObjects
  (params (InteractObjects :type Array%20of%20Interact%20Object%20Object%20References))
  (for (_array_element _array_index) InteractObjects
    (Utilities|Array|SetArrayElem (Variables|Default|GetInteractObjectsTransform) _array_index (Transformation|GetActorTransform _array_element))
    (Utilities|Array|SetArrayElem (Variables|Default|GetInteractObjectsEnergy) _array_index 0.0)))

(event Custom|UpdateEnemies
  (params (Enemies :type Array%20of%20Actor%20Object%20References))
  (for (_ _array_index) Enemies
    (Utilities|Array|SetArrayElem (Variables|Default|GetEnemiesTransform) _array_index 0.0)
    (Utilities|Array|SetArrayElem (Variables|Default|GetEnemiesHp) _array_index 0.0)))

(event Custom|Save
  (bind _returnvalue (SaveGame|CreateSaveGameObject "BP_SaveData_C"))
  (SaveGame|SaveGametoSlot _returnvalue "GameData"))