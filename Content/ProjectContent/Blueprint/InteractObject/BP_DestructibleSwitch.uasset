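; BP_DestructibleSwitch is a switch that breaks destructible objects and removes a blocking collision actor when turned on.
; Turn-on runs the parent logic, destroys BlockedCollision, then applies radius damage with impulse at each BombObject's own location, zeroing the PointLight inside that loop.
; Turn-off is overridden empty, and a Light timeline meant to modulate the light's intensity while inactive never runs.
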(event EventTurnOff
  (params (character :type Player%20Character%20Object%20Reference)))

(event EventTurnon
  (params (character :type Player%20Character%20Object%20Reference))
  (bind _blockedcollision (Variables|Default|GetBlockedCollision))
  (|CallParentFunction character)
  (if (Utilities|IsValid _blockedcollision)
    (Actor|DestroyActor _blockedcollision))
  (for _array_element (Variables|Default|GetBombObject)
    (Class|DestructibleComponent|ApplyRadiusDamage (Variables|/Script/ApexDestruction.DestructibleActor|GetDestructibleComponent _array_element) 3e+01 (Transformation|GetActorLocation _array_element) 1e+03 4e+03 false)
    (Rendering|Components|Light|SetIntensity (Variables|Default|GetPointLight) 0.0)))

(fn ConstructionScript)