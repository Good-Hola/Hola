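; BP_UpSlidingDoor is an interactable door that slides vertically when turned on.
; On BeginPlay it stores its root's world location as the default position.
; Turn on runs the parent behavior, then plays the DoorMove timeline, whose curve lerps the root's Z from that default up by MoveDist.
; The graph defines no reverse or closing motion.
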(event EventTurnon
  (params (character :type Player%20Character%20Object%20Reference))
  (bind _defaultlocation (Variables|Default|GetDefaultLocation))
  (|CallParentFunction character)
  (bind _doorcurve (Timeline|DoorMove Play)
    (:Update
      (Transformation|SetWorldLocation (Variables|Transformation|GetRootComponent) (Math|Vector|MakeVector (.x _defaultlocation) (.y _defaultlocation) (Math|Float|Lerp (.z _defaultlocation) (+ (.z _defaultlocation) (Variables|Default|GetMoveDist)) _doorcurve)) false false))))

(event EventBeginPlay
  (|CallParentFunction)
  (Variables|Default|SetDefaultLocation (Transformation|GetWorldLocation (Variables|Transformation|GetRootComponent))))

(fn ConstructionScript)