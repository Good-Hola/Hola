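; Sliding door interact object that moves toward a target actor's position when turned on and back when turned off.
; BeginPlay caches the root component's relative location as the closed position.
; Turn-on and turn-off call the parent logic, then play or reverse the DoorMove timeline.
; Its curve lerps the root's world location between the cached position and TargetLocation, without sweeping.
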(event EventTurnon
  (params (character :type Player%20Character%20Object%20Reference))
  (|CallParentFunction character)
  (bind _doorcurve (Timeline|DoorMove Play)
    (:Update
      (Transformation|SetWorldLocation (Variables|Transformation|GetRootComponent) (Math|Vector|Lerp(Vector) (Variables|Default|GetDefaultLocation) (Transformation|GetActorLocation (Variables|Default|GetTargetLocation)) _doorcurve) false false))))

(event EventTurnOff
  (params (character :type Player%20Character%20Object%20Reference))
  (|CallParentFunction character)
  (bind _doorcurve (Timeline|DoorMove Reverse)
    (:Update
      (Transformation|SetWorldLocation (Variables|Transformation|GetRootComponent) (Math|Vector|Lerp(Vector) (Variables|Default|GetDefaultLocation) (Transformation|GetActorLocation (Variables|Default|GetTargetLocation)) _doorcurve) false false))))

(event EventBeginPlay
  (|CallParentFunction)
  (Variables|Default|SetDefaultLocation (Variables|/Script/Engine.SceneComponent|GetRelativeLocation (Variables|Transformation|GetRootComponent))))

(fn ConstructionScript)