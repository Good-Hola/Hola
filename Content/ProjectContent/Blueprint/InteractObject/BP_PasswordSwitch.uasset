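; BP_PasswordSwitch is an interactable switch that contributes one piece of a password to a puzzle.
; On turn-on it runs the parent logic, then, if IsAct is set, adds its PeaceOfPassword value to the PasswordManager and turns its point light blue.
; ChangeLight sets the light to red-orange but is not called within this Blueprint, and the TurnOff event is empty.
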(event EventTurnOff
  (params (character :type Player%20Character%20Object%20Reference)))

(event EventTurnon
  (params (character :type Player%20Character%20Object%20Reference))
  (|CallParentFunction character)
  (if (Variables|Default|GetisAct)
    (Default|AddPassword (Variables|Default|GetPasswordManager) (Variables|Default|GetPeaceOfPassword))
    (Rendering|Components|Light|SetLightColor (Variables|Default|GetPointLight) "(R=0.246112,G=0.391275,B=0.994792,A=1.000000)" false)))

(fn ConstructionScript)

(fn ChangeLight
  (Rendering|Components|Light|SetLightColor (Variables|Default|GetPointLight) "(R=1.000000,G=0.097587,B=0.016807,A=1.000000)" true))