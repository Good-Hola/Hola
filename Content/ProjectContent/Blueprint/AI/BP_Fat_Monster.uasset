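; BP_Fat_Monster is an AI enemy character that melee-attacks the player, reacts to hits and ragdolls on death.
; MeleeAttack plays a random attack montage section, whose notifies sphere-trace from the matching hand socket to damage the player.
; Non-lethal damage plays a random hit reaction, then reports the damage to AI perception and stops the attack montage.
; Lethal damage unpossesses the AI controller, halts movement and enables delayed physics simulation.
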(event EventMeleeAttack
  (bind _mesh (Variables|Character|GetMesh))
  (bind _damage (Variables|기본/디폴트|GetDamage))
  (bind _mesh_2 (Variables|Character|GetMesh))
  (bind _returnvalue (Transformation|GetSocketLocation _mesh_2 "hand_r_socket"))
  (bind _returnvalue_2 (Transformation|GetSocketLocation _mesh "hand_l_socket"))
  ;[1 1 1] attack
  (bind _notifyname (Animation|Montage|PlayMontage (Variables|Character|GetMesh) "/Game/ProjectContent/AI/Animations/Fat_Monster_Attack_Montage.Fat_Monster_Attack_Montage" 1.0 0.0 (Utilities|String|StringToName (Utilities|Array|Get(acopy) (Variables|Default|GetAIMontageSection) (Math|Random|RandomIntegerinRange 3 4))))
    (:OnNotifyBegin
      (if (Utilities|Name|Equal(Name) _notifyname "leftAttackNotify")
        (bind _outhit (Collision|SphereTraceByChannel _returnvalue_2 (+ _returnvalue_2 (* (Math|Vector|GetForwardVector (Transformation|GetActorRotation)) 5e+01)) 4e+01 "TraceTypeQuery1" false 0 "None"))
        (Game|Damage|ApplyDamage (.AsPlayer%20Character (Utilities|Casting|CastToPlayerCharacter (.hitactor _outhit))) _damage 0 0)
        (Development|PrintString "Hit" (.bSuccess (Utilities|Casting|CastToPlayerCharacter (.hitactor _outhit))))
        (else
          (bind _outhit_2 (Collision|SphereTraceByChannel _returnvalue (+ _returnvalue (* (Math|Vector|GetForwardVector (Transformation|GetActorRotation)) 5e+01)) 4e+01 "TraceTypeQuery1" false 0 "None"))
          (Game|Damage|ApplyDamage (.AsPlayer%20Character (Utilities|Casting|CastToPlayerCharacter (.hitactor _outhit_2))) _damage 0 0)
          (Development|PrintString "Hit" (.bSuccess (Utilities|Casting|CastToPlayerCharacter (.hitactor _outhit_2)))))))))

(event Game|Damage|EventAnyDamage
  (params (Damage :type Float%20%28single-precision%29) (DamageType :type Damage%20Type%20Object%20Reference) (InstigatedBy :type Controller%20Object%20Reference) (DamageCauser :type Actor%20Object%20Reference))
  ;[1 1 1] apply damage
  (bind _output_get (Variables|Default|SetHP (- (Variables|Default|GetHP) Damage)))
  (if (<= _output_get 0.0)
    ;;[1 1 1] Death
    (Variables|Default|SetisAlive false)
    (bind _asbp_fat_monster_ai (Utilities|Casting|CastToBP_Fat_Monster_AI (Pawn|GetController)))
    (Pawn|UnPossess _asbp_fat_monster_ai)
    (Components|Movement|StopMovementImmediately (Variables|Character|GetCharacterMovement))
    (Collision|SetCollisionProfileName (Variables|Character|GetMesh) "Ragdoll" true :!class /Script/Engine.PrimitiveComponent)
    (Collision|SetCollisionEnabled (Variables|Collision|GetCapsuleComponent) "PhysicsOnly")
    (Utilities|FlowControl|Delay 1.0)
    (Physics|SetSimulatePhysics (Variables|Character|GetMesh) true)
    (else
      (Animation|PlayAnimMontage "/Game/ProjectContent/AI/Animations/Fat_Monster_Take_Damage_Montage.Fat_Monster_Take_Damage_Montage" 1.0 (Utilities|String|StringToName (Utilities|Array|Get(acopy) (Variables|Default|GetAIMontageSection) (Math|Random|RandomInteger 3))))
      (Utilities|FlowControl|Delay 0.5)
      (Class|AISenseDamage|ReportDamageEvent self DamageCauser Damage (Transformation|GetActorLocation) "0, 0, 0" "None")
      (Animation|StopAnimMontage "/Game/ProjectContent/AI/Animations/Fat_Monster_Attack_Montage.Fat_Monster_Attack_Montage"))))

(fn ConstructionScript)