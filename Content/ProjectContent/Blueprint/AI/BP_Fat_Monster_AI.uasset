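; AI controller for the fat monster that runs BT_Monster to drive patrolling, player detection and investigation.
; On BeginPlay it seeds the blackboard with patrol settings from the pawn's PatrolPath, or random-movement fallbacks, plus the initial chase state.
; Perception updates map stimuli by array index: the first sets CanSeePlayer, while successful second or third ones set IsInvestigating and Location.
; The Sensing function is an empty loop with disconnected duplicate logic.
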(event OnPerceptionUpdated(AIPerception)
  (params (UpdatedActors :type Array%20of%20Actor%20Object%20References))
  (bind _returnvalue (AI|GetBlackboard 0))
  (for _array_element UpdatedActors
    (bind _info (Class|AIPerceptionComponent|GetActorsPerception (Variables|Default|GetAIPerception) _array_element))
    (for (_array_element_2 _array_index) (.lastsensedstimuli _info)
      (bind _mypawn (Variables|Default|GetMyPawn)
        (:then
          (switch int _array_index
            (:0
              (AI|Components|Blackboard|SetValueasBool (AI|GetBlackboard 0) (Utilities|Name|MakeLiteralName "CanSeePlayer") (.bSuccessfullySensed (Utilities|Struct|BreakAIStimulus _array_element_2))))
            (:1
              (if (.bSuccessfullySensed (Utilities|Struct|BreakAIStimulus _array_element_2)) :!label _label
                (AI|Components|Blackboard|SetValueasBool _returnvalue (Utilities|Name|MakeLiteralName "IsInvestigating") (.bSuccessfullySensed (Utilities|Struct|BreakAIStimulus _array_element_2)))
                (AI|Components|Blackboard|SetValueasVector _returnvalue (Utilities|Name|MakeLiteralName "Location") (.StimulusLocation (Utilities|Struct|BreakAIStimulus _array_element_2)))))
            (:2
              (goto _label))))
        (:else)))))

(event EventBeginPlay
  (bind _returnvalue (AI|GetBlackboard 0))
  (bind _returnvalue_2 (Utilities|Name|MakeLiteralName "WaitTime"))
  (bind _returnvalue_3 (AI|GetBlackboard 0))
  (AI|RunBehaviorTree "/Game/ProjectContent/AI/AI/BT_Monster.BT_Monster")
  (bind _asbp_fat_monster (Utilities|Casting|CastToBP_Fat_Monster (Pawn|GetControlledPawn)))
  (bind _output_get (Variables|Default|SetMyPawn _asbp_fat_monster))
  (bind _patrolpath (Variables|/Game/ProjectContent/Blueprint/AI/BP_Fat_Monster.BP_Fat_Monster_C|GetPatrolPath _output_get)
    (:then
      (AI|Components|Blackboard|SetValueasBool _returnvalue_3 (Utilities|Name|MakeLiteralName "PathLooping") (Variables|/Game/ProjectContent/Blueprint/AI/PatrolPath.PatrolPath_C|GetisLooping _patrolpath))
      (AI|Components|Blackboard|SetValueasFloat _returnvalue_3 _returnvalue_2 (Variables|/Game/ProjectContent/Blueprint/AI/PatrolPath.PatrolPath_C|GetWaitTime _patrolpath)))
    (:else
      (AI|Components|Blackboard|SetValueasBool _returnvalue (Utilities|Name|MakeLiteralName "PathLooping") (Variables|/Game/ProjectContent/Blueprint/AI/BP_Fat_Monster.BP_Fat_Monster_C|GetRandomMoving (Variables|Default|GetMyPawn)))
      (AI|Components|Blackboard|SetValueasFloat _returnvalue _returnvalue_2 3.0)))
  (Class|BlackboardComponent|SetValueasInt (AI|GetBlackboard 0) (Utilities|Name|MakeLiteralName "Direction") 1)
  (Variables|Default|SetCurrentTarget (Game|GetPlayerCharacter 0))
  (AI|Components|Blackboard|SetValueasEnum (AI|GetBlackboard 0) (Utilities|Name|MakeLiteralName "ChaseStatus") (Variables|Default|GetCurrentState)))

(fn ConstructionScript)

(fn Sensing
  (params (Array :type Array%20of%20AI%20Stimulus%20Structures))
  (for _array_element Array
    _))